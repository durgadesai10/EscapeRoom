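; Rotatable painting puzzle piece that unlocks a BP_SolvedPainting_Opens actor once every painting in the level is correctly oriented.
; Interacting turns the frame a quarter turn with a randomized slide sound, then compares its wrapped position index to PuzzleAnswer to set Finalized.
; Each instance polls all paintings on a looping timer, and when all are finalized stops its timer, blocks further rotation and calls UnlockPainting.
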(event Custom|RotatePainting
  (bind _pictureframe (Variables|Default|GetPictureFrame))
  (if (not (Variables|Default|GetFrameMoving))
    (Variables|Default|SetFrameMoving true)
    (Audio|PlaySound2D "/Game/Game/Sounds/WoodSlide.WoodSlide" (Math|Random|RandomFloatinRange 0.5 1.5) (Math|Random|RandomFloatinRange 0.8 1.2) 0.0 0 0)
    (Components|MoveComponentTo _pictureframe "0, 0, 0" (Math|Rotator|CombineRotators (Variables|/Script/Engine.SceneComponent|GetRelativeRotation _pictureframe) "-90.000000,0.000000,0.000000") true true 1.0 true)
    (Variables|Default|SetFrameMoving false)
    (bind _result (Math|Integer|IncrementInt (Variables|Default|GetFramePosition))
      (:%20%20
        (Variables|Default|SetFramePosition _result)
        (CallFunction|PaintingCheck)))))

(event Custom|PaintingCheck
  (if (> (Variables|Default|GetFramePosition) 3)
    (Variables|Default|SetFramePosition 0))
  (if (== (Variables|Default|GetFramePosition) (Variables|Default|GetPuzzleAnswer))
    (Development|PrintString "Puzzle Solved" true true "(R=0.000000,G=1.000000,B=0.240638,A=1.000000)")
    (Variables|Default|SetFinalized true)
    (else
      (Variables|Default|SetFinalized false)
      (Development|PrintString "Puzzle Unfinalized" true true "(R=1.000000,G=0.000000,B=0.000000,A=1.000000)"))))

(event Custom|PuzzleCheck
  (Variables|Default|SetPuzzleSolved true)
  (for _array_element (Variables|Default|GetAllPaintings)
    (if (not (Variables|BP_Painting_MasterPuzzle_C|GetFinalized _array_element))
      (Variables|Default|SetPuzzleSolved false)))
  (if (Variables|Default|GetPuzzleSolved)
    (Utilities|Time|ClearandInvalidateTimerbyHandle (stale EventBeginPlay _returnvalue_2))
    (Default|UnlockPainting (Variables|Default|GetTriggeredPainting))))

(event EventInteractwith
  (params (PlayerCharacter :type BP%20First%20Person%20Character%20Object%20Reference))
  (if (not (Variables|Default|GetPuzzleSolved))
    (CallFunction|RotatePainting)))

(event EventTick
  (params (DeltaSeconds :type Float%20%28single-precision%29))
  (Development|PrintString (Utilities|String|ToString(Integer) (Variables|Default|GetFramePosition)) true true "(R=0.000000,G=0.660000,B=1.000000,A=1.000000)" DeltaSeconds))

(event EventBeginPlay
  (bind _outactors (Actor|GetAllActorsOfClass "BP_Painting_MasterPuzzle_C"))
  (Variables|Default|SetAllPaintings _outactors)
  (bind _returnvalue (Actor|GetActorOfClass "/Game/Game/Blueprints/BP_SolvedPainting_Opens.BP_SolvedPainting_Opens_C"))
  (Variables|Default|SetTriggeredPainting _returnvalue)
  (bind _returnvalue_2 (Utilities|Time|SetTimerbyEvent (delegate Custom|PuzzleCheck) 0.25 true)))

(fn ConstructionScript)

(fn Lookat
  (return "" ""))