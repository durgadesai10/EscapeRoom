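; BP_SciFi_Switch is an interactable wall switch whose handle starts hidden until the player supplies it.
; Interacting shows the handle once the player's inventory query finds the required item.
; Later interactions use a FlipFlop to ease the handle between two rotations.
; If the assigned switchboard is solved, a flip also unlocks and toggles the assigned door, if still locked, and turns the assigned light green.
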(event EventBeginPlay
  (Rendering|SetVisibility (Variables|Default|GetSciFi_Switch_Handle) false false))

(event EventInteractwith
  (params (PlayerCharacter :type BP%20First%20Person%20Character%20Object%20Reference))
  (bind _scifi_switch_handle (Variables|Default|GetSciFi_Switch_Handle))
  (bind _assigneddoor (Variables|Default|GetAssignedDoor))
  (if (Variables|Default|GetHandlePlaced)
    (Utilities|FlowControl|FlipFlop
      (:A
        (Components|MoveComponentTo _scifi_switch_handle "0, 0, 0" "160.000000,0.000000,0.000000" false true 2.0 true)
        (Variables|Default|SetFinished true))
      (:B
        (Components|MoveComponentTo _scifi_switch_handle "0, 0, 0" "-10.000000,0.000000,0.000000" false true 2.0 true)))
    (if (not (Variables|/Game/Game/Blueprints/BP_WoodenDoor.BP_WoodenDoor_C|GetDoorUnlocked _assigneddoor))
      (if (Variables|/Game/Game/Blueprints/BP_SwitchBox_Puzzle.BP_SwitchBox_Puzzle_C|GetIsSolved (Variables|Default|GetAssignedSwitchboard))
        (Variables|/Game/Game/Blueprints/BP_WoodenDoor.BP_WoodenDoor_C|SetDoorUnlocked _assigneddoor true)
        (Default|OpenCloseDoor _assigneddoor)
        (Default|GlowGreen (Variables|Default|GetAssignedLight))))
    (else
      (bind _requiredhandle (Variables|Default|GetRequiredHandle)
        (:then
          (bind _return (Default|QueryInventory (Variables|/Game/FirstPerson/Blueprints/BP_FirstPersonCharacter.BP_FirstPersonCharacter_C|GetInventorySystem PlayerCharacter) _requiredhandle 1))
          (if _return
            (Rendering|SetVisibility (Variables|Default|GetSciFi_Switch_Handle) true false)
            (Variables|Default|SetHandlePlaced true)))
        (:else)))))

(fn ConstructionScript)

(fn Lookat
  (return "" ""))