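; Puzzle painting that swings open like a door once solved, then can be toggled open and closed by the player.
; UnlockPainting plays click and creak sounds at the frame, eases it to the open rotation and sets IsUnlocked and IsOpen.
; Interactwith works only when unlocked, toggling the frame with MoveComponentTo, though its creak plays at world origin.
; LookAt returns an empty verb and noun.
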(event Custom|UnlockPainting
  (bind _paintingframe (Variables|Default|GetPaintingFrame))
  (bind _returnvalue (Transformation|GetWorldLocation _paintingframe))
  (Audio|PlaySoundatLocation "/Game/Game/Sounds/117042__joedeshon__power_door_click_01.117042__joedeshon__power_door_click_01" _returnvalue "0, 0, 0" 0.5 1.0 0.0 0 0 0 0)
  (Audio|PlaySoundatLocation "/Game/Game/Sounds/458049__quetzalcontla__door-creaking.458049__quetzalcontla__door-creaking" _returnvalue "0, 0, 0" 1.0 1.0 0.0 0 0 0 0)
  (Components|MoveComponentTo (Variables|Default|GetPaintingFrame) (Variables|/Script/Engine.SceneComponent|GetRelativeLocation _paintingframe) "0.000000,0.000000,40.000000" true true 2.0 true)
  (Variables|Default|SetisOpen true)
  (Variables|Default|SetisUnlocked true))

(event EventBeginPlay)

(event Collision|EventActorBeginOverlap
  (params (OtherActor :type Actor%20Object%20Reference)))

(event EventTick
  (params (DeltaSeconds :type Float%20%28single-precision%29)))

(event EventInteractwith
  (params (PlayerCharacter :type BP%20First%20Person%20Character%20Object%20Reference))
  (bind _paintingframe (Variables|Default|GetPaintingFrame))
  (bind _relativelocation (Variables|/Script/Engine.SceneComponent|GetRelativeLocation _paintingframe))
  (if (Variables|Default|GetisUnlocked)
    (Audio|PlaySoundatLocation "/Game/Game/Sounds/458049__quetzalcontla__door-creaking.458049__quetzalcontla__door-creaking" "0, 0, 0" "0, 0, 0" 1.0 1.0 0.0 0 0 0 0)
    (if (Variables|Default|GetisOpen)
      (Components|MoveComponentTo _paintingframe _relativelocation "0, 0, 0" true true 2.0 true)
      (Variables|Default|SetisOpen false)
      (else
        (Components|MoveComponentTo _paintingframe _relativelocation "0.000000,0.000000,40.000000" true true 2.0 true)
        (Variables|Default|SetisOpen true)))))

(fn ConstructionScript)

(fn Lookat
  (return "" ""))