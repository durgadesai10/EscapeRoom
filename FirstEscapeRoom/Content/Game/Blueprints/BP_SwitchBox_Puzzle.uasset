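; Switch box puzzle where the player toggles four clickable switches to turn four red lights green.
; Interacting blends to or from a close-up view, swapping movement, look and flashlight for cursor clicks and a spotlight.
; Each switch flips a fixed group of light booleans, which Tick mirrors to visibility.
; When all are green, Tick notifies BP_LightOverFirstDoor, blocks further interaction and exits the close-up, repeating this every frame.
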(event OnClicked(Switch_01)
  (params (TouchedComponent :type Primitive%20Component%20Object%20Reference) (ButtonPressed :type Key%20Structure :default "None"))
  (bind _switchlight_01_red (Variables|Default|GetSwitchLight_01_Red))
  (bind _switchlight_01_green (Variables|Default|GetSwitchLight_01_Green))
  (bind _switch_01 (Variables|Default|GetSwitch_01))
  ;[0.15 0.15 0.15 0.5] Switch 1 - Controls L1 and L4
  (Development|PrintString "Switch 1 Clicked")
  (Variables|Default|SetL1isGreen (not (Variables|Default|GetL1isGreen)))
  (Variables|Default|SetL4isGreen (not (Variables|Default|GetL4isGreen)))
  (Utilities|FlowControl|FlipFlop
    (:A
      (Transformation|SetRelativeRotation _switch_01 "180.000000,0.000000,0.000000" false false)
      (Rendering|SetVisibility _switchlight_01_red false false)
      (Rendering|SetVisibility _switchlight_01_green true false))
    (:B
      (Transformation|SetRelativeRotation _switch_01 "0, 0, 0" false false)
      (Rendering|SetVisibility _switchlight_01_red true false)
      (Rendering|SetVisibility _switchlight_01_green false false))))

(event OnClicked(Switch_02)
  (params (TouchedComponent :type Primitive%20Component%20Object%20Reference) (ButtonPressed :type Key%20Structure :default "None"))
  (bind _switch_02 (Variables|Default|GetSwitch_02))
  (bind _switchlight_02_red (Variables|Default|GetSwitchLight_02_Red))
  (bind _switchlight_02_green (Variables|Default|GetSwitchLight_02_Green))
  ;[0.15 0.15 0.15 0.5] Switch 2 - Controls L1, L2, and L3
  (Development|PrintString "Switch 2 Clicked")
  (Variables|Default|SetL1isGreen (not (Variables|Default|GetL1isGreen)))
  (Variables|Default|SetL2isGreen (not (Variables|Default|GetL2isGreen)))
  (Variables|Default|SetL3isGreen (not (Variables|Default|GetL3isGreen)))
  (Utilities|FlowControl|FlipFlop
    (:A
      (Transformation|SetRelativeRotation _switch_02 "180.000000,0.000000,0.000000" false false)
      (Rendering|SetVisibility _switchlight_02_red false false)
      (Rendering|SetVisibility _switchlight_02_green true false))
    (:B
      (Transformation|SetRelativeRotation _switch_02 "0, 0, 0" false false)
      (Rendering|SetVisibility _switchlight_02_red true false)
      (Rendering|SetVisibility _switchlight_02_green false false))))

(event OnClicked(Switch_03)
  (params (TouchedComponent :type Primitive%20Component%20Object%20Reference) (ButtonPressed :type Key%20Structure :default "None"))
  (bind _switch_03 (Variables|Default|GetSwitch_03))
  (bind _switchlight_03_green (Variables|Default|GetSwitchLight_03_Green))
  (bind _switchlight_03_red (Variables|Default|GetSwitchLight_03_Red))
  ;[0.15 0.15 0.15 0.5] Switch 3 - Controls L3 and L4
  (Development|PrintString "Switch 3 Clicked")
  (Variables|Default|SetL3isGreen (not (Variables|Default|GetL3isGreen)))
  (Variables|Default|SetL4isGreen (not (Variables|Default|GetL4isGreen)))
  (Utilities|FlowControl|FlipFlop
    (:A
      (Transformation|SetRelativeRotation _switch_03 "180.000000,0.000000,0.000000" false false)
      (Rendering|SetVisibility _switchlight_03_red false false)
      (Rendering|SetVisibility _switchlight_03_green true false))
    (:B
      (Transformation|SetRelativeRotation _switch_03 "0, 0, 0" false false)
      (Rendering|SetVisibility _switchlight_03_red true false)
      (Rendering|SetVisibility _switchlight_03_green false false))))

(event OnClicked(Switch_04)
  (params (TouchedComponent :type Primitive%20Component%20Object%20Reference) (ButtonPressed :type Key%20Structure :default "None"))
  (bind _switch_04 (Variables|Default|GetSwitch_04))
  (bind _switchlight_04_green (Variables|Default|GetSwitchLight_04_Green))
  (bind _switchlight_04_red (Variables|Default|GetSwitchLight_04_Red))
  ;[0.15 0.15 0.15 0.5] Switch 4 - Controls L2 and L4
  (Development|PrintString "Switch 4 Clicked")
  (Variables|Default|SetL2isGreen (not (Variables|Default|GetL2isGreen)))
  (Variables|Default|SetL4isGreen (not (Variables|Default|GetL4isGreen)))
  (Utilities|FlowControl|FlipFlop
    (:A
      (Transformation|SetRelativeRotation _switch_04 "180.000000,0.000000,0.000000" false false)
      (Rendering|SetVisibility _switchlight_04_red false false)
      (Rendering|SetVisibility _switchlight_04_green true false))
    (:B
      (Transformation|SetRelativeRotation _switch_04 "0, 0, 0" false false)
      (Rendering|SetVisibility _switchlight_04_red true false)
      (Rendering|SetVisibility _switchlight_04_green false false))))

(event EventBeginPlay
  (bind _asbp_first_person_character (Utilities|Casting|CastToBP_FirstPersonCharacter (Game|GetPlayerCharacter 0)))
  (Variables|Default|SetPlayerRef _asbp_first_person_character)
  (Input|EnableInput (Game|GetPlayerController 0))
  (Actor|GetAllActorsOfClass "/Game/FirstPerson/Blueprints/BP_FirstPersonCharacter.BP_FirstPersonCharacter_C")
  (bind _returnvalue (Actor|GetActorOfClass "/Game/Game/Blueprints/BP_LightOverFirstDoor.BP_LightOverFirstDoor_C"))
  (Variables|Default|SetLightOverDoor _returnvalue))

(event EventTick
  (params (DeltaSeconds :type Float%20%28single-precision%29))
  (bind _returnvalue (Game|GetPlayerController 0))
  (bind _playerref (Variables|Default|GetPlayerRef))
  (bind _light_01_red (Variables|Default|GetLight_01_Red))
  (bind _light_01_green (Variables|Default|GetLight_01_Green))
  (bind _light_02_red (Variables|Default|GetLight_02_Red))
  (bind _light_02_green (Variables|Default|GetLight_02_Green))
  (bind _light_03_red (Variables|Default|GetLight_03_Red))
  (bind _light_03_green (Variables|Default|GetLight_03_Green))
  (bind _light_04_green (Variables|Default|GetLight_04_Green))
  (bind _light_04_red (Variables|Default|GetLight_04_Red))
  ;[0.15 0.15 0.15 0.5] Light Activation
  (if (Variables|Default|GetL1isGreen)
    (Rendering|SetVisibility _light_01_red false false)
    (Rendering|SetVisibility _light_01_green true false)
    (else
      (Rendering|SetVisibility _light_01_red true false)
      (Rendering|SetVisibility _light_01_green false false)))
  (if (Variables|Default|GetL2isGreen)
    (Rendering|SetVisibility _light_02_red false false)
    (Rendering|SetVisibility _light_02_green true false)
    (else
      (Rendering|SetVisibility _light_02_red true false)
      (Rendering|SetVisibility _light_02_green false false)))
  (if (Variables|Default|GetL3isGreen)
    (Rendering|SetVisibility _light_03_red false false)
    (Rendering|SetVisibility _light_03_green true false)
    (else
      (Rendering|SetVisibility _light_03_red true false)
      (Rendering|SetVisibility _light_03_green false false)))
  (if (Variables|Default|GetL4isGreen)
    (Rendering|SetVisibility _light_04_red false false)
    (Rendering|SetVisibility _light_04_green true false)
    (else
      (Rendering|SetVisibility _light_04_red true false)
      (Rendering|SetVisibility _light_04_green false false)))
  (if (Math|Boolean|ANDBoolean (Variables|Default|GetL1isGreen) (Variables|Default|GetL2isGreen) (Variables|Default|GetL3isGreen) (Variables|Default|GetL4isGreen))
    (Rendering|SetVisibility (Variables|/Script/Engine.Light|GetLightComponent (Variables|Default|GetActivatedLight)) true false)
    (Default|SwitchboxSolved (Variables|Default|GetLightOverDoor))
    (Variables|Default|SetIsSolved true)
    ;[0.15 0.15 0.15 0.5] Interaction with Switch Box - Camera Close Up
    (Variables|Default|SetInCloseUp false)
    (Game|Player|SetViewTargetwithBlend (Game|GetPlayerController 0) (Variables|Default|GetPlayerRef) 0.5 "VTBlend_Linear" 0.0 true)
    (Variables|/Script/Engine.PlayerController|SetbEnableClickEvents _returnvalue false)
    (Variables|/Script/Engine.PlayerController|SetbShowMouseCursor _returnvalue false)
    (Pawn|Components|CharacterMovement|SetMovementMode (Variables|/Script/Engine.Character|GetCharacterMovement (Variables|Default|GetPlayerRef)) "MOVE_Walking" 0)
    (Input|SetIgnoreLookInput _returnvalue false)
    (Rendering|SetVisibility (Variables|Default|GetSpotLight) false false)
    (if (Variables|/Game/FirstPerson/Blueprints/BP_FirstPersonCharacter.BP_FirstPersonCharacter_C|GetFlashlightIsOn _playerref)
      (Rendering|SetVisibility (Variables|/Game/FirstPerson/Blueprints/BP_FirstPersonCharacter.BP_FirstPersonCharacter_C|Getflashlight _playerref) true false))))

(event EventInteractwith
  (params (PlayerCharacter :type BP%20First%20Person%20Character%20Object%20Reference))
  (bind _returnvalue (Game|GetPlayerController 0))
  (bind _playerref (Variables|Default|GetPlayerRef))
  (bind _flashlightison (Variables|/Game/FirstPerson/Blueprints/BP_FirstPersonCharacter.BP_FirstPersonCharacter_C|GetFlashlightIsOn _playerref))
  (bind _flashlight (Variables|/Game/FirstPerson/Blueprints/BP_FirstPersonCharacter.BP_FirstPersonCharacter_C|Getflashlight _playerref))
  ;[0.15 0.15 0.15 0.5] Interaction with Switch Box - Camera Close Up
  (if (not (Variables|Default|GetIsSolved))
    (if (Variables|Default|GetInCloseUp)
      (Variables|Default|SetInCloseUp false)
      (Game|Player|SetViewTargetwithBlend (Game|GetPlayerController 0) (Variables|Default|GetPlayerRef) 0.5 "VTBlend_Linear" 0.0 true)
      (Variables|/Script/Engine.PlayerController|SetbEnableClickEvents _returnvalue false)
      (Variables|/Script/Engine.PlayerController|SetbShowMouseCursor _returnvalue false)
      (Pawn|Components|CharacterMovement|SetMovementMode (Variables|/Script/Engine.Character|GetCharacterMovement (Variables|Default|GetPlayerRef)) "MOVE_Walking" 0)
      (Input|SetIgnoreLookInput _returnvalue false)
      (Rendering|SetVisibility (Variables|Default|GetSpotLight) false false)
      (if _flashlightison
        (Rendering|SetVisibility _flashlight true false))
      (else
        (Variables|Default|SetInCloseUp true)
        (Game|Player|SetViewTargetwithBlend _returnvalue self 0.5 "VTBlend_Linear" 0.0 true)
        (Variables|/Script/Engine.PlayerController|SetbEnableClickEvents _returnvalue true)
        (Variables|/Script/Engine.PlayerController|SetbShowMouseCursor _returnvalue true)
        (Pawn|Components|CharacterMovement|DisableMovement (Variables|/Script/Engine.Character|GetCharacterMovement (Variables|Default|GetPlayerRef)))
        (Input|SetIgnoreLookInput _returnvalue true)
        (Rendering|SetVisibility (Variables|Default|GetSpotLight) true false)
        (if _flashlightison
          (Rendering|SetVisibility _flashlight false false))))))

(fn ConstructionScript)

(fn Lookat
  (return "" ""))