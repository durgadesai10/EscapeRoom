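; Wooden door Blueprint that the player opens and closes by interacting with it while it is unlocked.
; A dot product between the player offset and the door's right vector picks the swing direction, then MoveComponentTo eases the door mesh open or back shut with creak and open/close sounds.
; An optional looping timer closes the door once the player moves beyond CloseDistance.
; Proximity-open logic is present but disconnected, and LookAt returns empty text.
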(event Custom|OpenCloseDoor
  (bind _self self)
  (bind _woodendoor_door (Variables|Default|GetWoodenDoor_Door))
  (bind _relativelocation (Variables|/Script/Engine.SceneComponent|GetRelativeLocation _woodendoor_door))
  ;[0.15 0.15 0.15 0.5] Open Close Logic
  (if (not (Variables|Default|GetOngoingAction))
    (if (Variables|Default|GetDoorUnlocked)
      (if (Variables|Default|GetDoorClosed)
        (Variables|Default|SetDotProduct (Math|Vector|DotProduct (Math|Vector|Normalize (- (Transformation|GetActorLocation _self) (Transformation|GetActorLocation (Variables|Default|GetPlayerRef)))) (Transformation|GetActorRightVector _self)))
        (Variables|Default|SetOngoingAction true)
        (if (< (Variables|Default|GetDotProduct) 0.0)
          (Variables|Default|SetDoorRotation "0.000000,100.000000,0.000000")
          (else
            (Variables|Default|SetDoorRotation "0.000000,-100.000000,0.000000")))
        (CallFunction|Sounds)
        (Audio|PlaySoundatLocation "/Game/Game/Sounds/DoorCreak.DoorCreak" _relativelocation "0, 0, 0" 1.0 5.0 0.0 0 0 0 0)
        (Components|MoveComponentTo _woodendoor_door _relativelocation (Variables|Default|GetDoorRotation) true true 2.0 true)
        (Variables|Default|SetDoorClosed false)
        (Variables|Default|SetOngoingAction false)
        (Development|PrintString "Open")
        (else
          (Development|PrintString "Closing Door")
          (Audio|PlaySoundatLocation "/Game/Game/Sounds/DoorCreak.DoorCreak" _relativelocation "0, 0, 0" 1.0 (Math|Random|RandomFloatinRange 0.5 1.8) 0.0 0 0 0 0)
          (Components|MoveComponentTo _woodendoor_door _relativelocation "0, 0, 0" true true 2.0 true)
          (CallFunction|Sounds)
          (Variables|Default|SetDoorClosed true)
          (Variables|Default|SetOngoingAction false)
          (Development|PrintString "Closed")))
      (else
        (Development|PrintString "Door Locked")))))

(event Custom|AutoClose
  ;[0.15 0.15 0.15 0.5] Auto Close Door
  (if (Variables|Default|GetAutoCloseFunctionality)
    (Utilities|Time|SetTimerbyEvent (delegate Custom|DoorAutoClose) 2.0 true true)))

(event Custom|DoorAutoClose
  ;[0.15 0.15 0.15 0.5] Auto Close Door
  (if (not (Variables|Default|GetDoorClosed))
    (if (> (Math|Vector|Distance(Vector) (Transformation|GetActorLocation (Variables|Default|GetPlayerRef)) (Transformation|GetActorLocation)) (Variables|Default|GetCloseDistance))
      (CallFunction|OpenCloseDoor))))

(event EventBeginPlay
  (bind _asbp_first_person_character (Utilities|Casting|CastToBP_FirstPersonCharacter (Game|GetPlayerCharacter 0)))
  (Variables|Default|SetPlayerRef _asbp_first_person_character)
  (CallFunction|AutoClose))

(event EventInteractwith
  (params (PlayerCharacter :type BP%20First%20Person%20Character%20Object%20Reference))
  (Development|PrintString "Door Clicked")
  (if (Variables|Default|GetDoorUnlocked)
    (CallFunction|OpenCloseDoor)))

(fn ConstructionScript)

(fn Sounds
  (bind _woodendoor_door (Variables|Default|GetWoodenDoor_Door))
  (bind _returnvalue (Transformation|GetWorldLocation _woodendoor_door))
  (if (Variables|Default|GetDoorUnlocked)
    (if (Variables|Default|GetDoorClosed)
      (Audio|PlaySoundatLocation (Variables|Default|GetOpenDoorSound) _returnvalue "0, 0, 0" 0.5 1.0 0.0 0 0 0 0)
      (else
        (Audio|PlaySoundatLocation (Variables|Default|GetCloseDoorSound) _returnvalue "0, 0, 0" 0.34 1.0 0.1 0 0 0 0)))))

(fn Lookat
  (return "" ""))