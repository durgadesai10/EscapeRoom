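; Sci-fi sliding double door that opens when a player interacts while carrying its required keycard.
; Interactwith queries the player's InventorySystem, then eases both panels apart with MoveComponentTo, offset from their current positions.
; Without a RequiredKeycard set it never opens, and no state guards against repeat opening.
; LookAt returns empty text; the Timeline and collision nodes are disconnected leftovers.
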(event Custom|OpenRightDoor
  (bind _scifidoor_right (Variables|Default|GetSciFiDoor_Right))
  (Components|MoveComponentTo _scifidoor_right (+ (Variables|/Script/Engine.SceneComponent|GetRelativeLocation _scifidoor_right) "100.000000,0.000000,0.000000") "0, 0, 0" true true 3.0 false))

(event Custom|OpenLeftDoor
  (bind _scifidoor_left (Variables|Default|GetSciFiDoor_Left))
  (Components|MoveComponentTo _scifidoor_left (+ (Variables|/Script/Engine.SceneComponent|GetRelativeLocation _scifidoor_left) "-100.000000,0.000000,0.000000") "0, 0, 0" true true 3.0 false))

(event EventBeginPlay)

(event Collision|EventActorBeginOverlap
  (params (OtherActor :type Actor%20Object%20Reference)))

(event EventTick
  (params (DeltaSeconds :type Float%20%28single-precision%29)))

(event EventInteractwith
  (params (PlayerCharacter :type BP%20First%20Person%20Character%20Object%20Reference))
  (bind _requiredkeycard (Variables|Default|GetRequiredKeycard)
    (:then
      (bind _return (Default|QueryInventory (Variables|/Game/FirstPerson/Blueprints/BP_FirstPersonCharacter.BP_FirstPersonCharacter_C|GetInventorySystem PlayerCharacter) _requiredkeycard 1))
      (if _return
        (CallFunction|OpenRightDoor)
        (CallFunction|OpenLeftDoor)))
    (:else)))

(fn ConstructionScript)

(fn Lookat
  (return "" ""))