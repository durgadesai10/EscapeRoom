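; BP_Pickup is an interactable world item, driven by a data asset, that the player picks up into the inventory system.
; The construction script sets its mesh from the data asset, and LookAt returns a "Pickup" prompt with the item name.
; Interacting adds the quantity to inventory; if that succeeds and the item is destroyed on pickup, it destroys itself, shows an obtained-object widget and disables any linked dialogue box's collision.
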(event Collision|EventActorBeginOverlap
  (params (OtherActor :type Actor%20Object%20Reference)))

(event EventTick
  (params (DeltaSeconds :type Float%20%28single-precision%29)))

(event EventInteractwith
  (params (PlayerCharacter :type BP%20First%20Person%20Character%20Object%20Reference))
  (bind _dataasset (Variables|Default|GetDataAsset))
  (bind _returnsuccess (Default|AddtoInventory (Variables|/Game/FirstPerson/Blueprints/BP_FirstPersonCharacter.BP_FirstPersonCharacter_C|GetInventorySystem PlayerCharacter) _dataasset (Variables|Default|GetQuantity)))
  (if (and _returnsuccess (Variables|/Game/Game/InventorySystem/Data/DA_Item.DA_Item_C|GetIsDestroyedOnPickup _dataasset))
    (Actor|DestroyActor)
    (bind _returnvalue (UserInterface|CreateWidget "/Game/Game/Widgets/WB_ObjectObtained.WB_ObjectObtained_C"))
    (Variables|/Game/Game/Widgets/WB_ObjectObtained.WB_ObjectObtained_C|SetObject_Name _returnvalue (Utilities|String|ToString(Text) (Variables|/Game/Game/InventorySystem/Data/DA_Item.DA_Item_C|GetName (Variables|Default|GetDataAsset))))
    (Default|AssignObject _returnvalue)
    (if (Variables|Default|GetHasDialogueBoxRef)
      (Collision|SetCollisionEnabled (Variables|/Game/Game/Blueprints/BP_DialogueBox.BP_DialogueBox_C|GetBox (Variables|Default|GetDialogueBoxRef)) "NoCollision"))))

(fn ConstructionScript
  (bind _dataasset (Variables|Default|GetDataAsset)
    (:then
      (Components|StaticMesh|SetStaticMesh (Variables|Default|GetStaticMesh) (Variables|/Game/Game/InventorySystem/Data/DA_Item.DA_Item_C|GetStaticMesh _dataasset)))
    (:else)))

(fn Lookat
  (return "Pickup" (Variables|/Game/Game/InventorySystem/Data/DA_Item.DA_Item_C|GetName (Variables|Default|GetDataAsset))))