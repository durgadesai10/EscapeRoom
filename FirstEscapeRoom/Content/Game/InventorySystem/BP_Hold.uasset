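; BP_Hold is a physics prop that the first-person character can pick up and drop, with its mesh taken from a data asset.
; Hold and release events attach it to the player's PhysicsHandle, while Tick adds a small force toward the handle's target.
; Collision toggles switch physics and grabbing on or off.
; ReturnToStart releases it and teleports it to the location recorded in the construction script.
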(event Custom|Grabbed
  (bind _staticmesh (Variables|Default|GetStaticMesh))
  (Physics|Components|PhysicsHandle|GrabComponentatLocationwithRotation (Variables|/Game/FirstPerson/Blueprints/BP_FirstPersonCharacter.BP_FirstPersonCharacter_C|GetPhysicsHandle (Variables|Default|GetPlayerRef)) _staticmesh "None" (Transformation|GetWorldLocation _staticmesh) "0, 0, 0")
  (Variables|Default|SetIsGrabbing true)
  (Development|PrintString "Grabbed"))

(event Custom|Released
  (if (Variables|Default|GetIsGrabbing)
    (Physics|Components|PhysicsHandle|ReleaseComponent (Variables|/Game/FirstPerson/Blueprints/BP_FirstPersonCharacter.BP_FirstPersonCharacter_C|GetPhysicsHandle (Variables|Default|GetPlayerRef)))
    (Variables|Default|SetIsGrabbing false)
    (Development|PrintString "Released")))

(event Custom|DisableCollision
  (bind _staticmesh (Variables|Default|GetStaticMesh))
  (Development|PrintString "Disable Collision")
  (Physics|SetSimulatePhysics _staticmesh false)
  (Collision|SetCollisionEnabled _staticmesh "QueryAndProbe")
  (Variables|Default|SetIsGrabEnabled false))

(event Custom|EnableCollision
  (bind _staticmesh (Variables|Default|GetStaticMesh))
  (Development|PrintString "Enabled Collision")
  (Physics|SetSimulatePhysics _staticmesh true)
  (Collision|SetCollisionEnabled _staticmesh "QueryAndPhysics")
  (Variables|Default|SetIsGrabEnabled true))

(event Custom|ReturnToStart
  (bind _staticmesh (Variables|Default|GetStaticMesh))
  (Transformation|SetWorldLocation (Variables|Default|GetStaticMesh) (Variables|Default|GetStartingLocation) false true)
  (CallFunction|ReleaseObject)
  (Development|PrintString "Object Gone" true true "(R=1.000000,G=0.781819,B=0.000000,A=1.000000)")
  (Physics|SetSimulatePhysics _staticmesh true)
  (Collision|SetCollisionEnabled _staticmesh "QueryAndPhysics"))

(event EventBeginPlay
  (bind _asbp_first_person_character (Utilities|Casting|CastToBP_FirstPersonCharacter (Game|GetPlayerCharacter 0)))
  (Variables|Default|SetPlayerRef _asbp_first_person_character)
  (Development|PrintString (Utilities|String|ToString(Vector) (Variables|Default|GetStartingLocation)) true true "(R=0.000000,G=0.660000,B=1.000000,A=1.000000)" 3.0))

(event EventHoldObject
  (params (PlayerCharacter :type BP%20First%20Person%20Character%20Object%20Reference))
  (if (Variables|Default|GetIsGrabEnabled)
    (CallFunction|Grabbed)))

(event EventReleaseObject
  (params (PlayerRef :type BP%20First%20Person%20Character%20Object%20Reference))
  (if (Variables|Default|GetIsGrabEnabled)
    (Variables|Default|SetReleasedKey true)
    (CallFunction|Released)))

(event EventTick
  (params (DeltaSeconds :type Float%20%28single-precision%29))
  (bind _staticmesh (Variables|Default|GetStaticMesh))
  (if (Variables|Default|GetIsGrabbing)
    (Physics|AddForce _staticmesh (* "2.000000,2.000000,2.000000" (Math|Vector|Normalize (- (.TargetLocation (Class|PhysicsHandleComponent|GetTargetLocationandRotation (Variables|/Game/FirstPerson/Blueprints/BP_FirstPersonCharacter.BP_FirstPersonCharacter_C|GetPhysicsHandle (Variables|Default|GetPlayerRef)))) (Transformation|GetWorldLocation _staticmesh)))) "None" false)))

(event Collision|EventActorBeginOverlap
  (params (OtherActor :type Actor%20Object%20Reference)))

(fn ConstructionScript
  (bind _staticmesh (Variables|Default|GetStaticMesh))
  (bind _dataasset (Variables|Default|GetDataAsset)
    (:then
      (Components|StaticMesh|SetStaticMesh _staticmesh (Variables|/Game/Game/InventorySystem/Data/DA_Item.DA_Item_C|GetStaticMesh _dataasset))
      (Physics|SetSimulatePhysics _staticmesh true)
      (Class|PrimitiveComponent|SetUseCCD _staticmesh true "None")
      (Variables|Default|SetStartingLocation (Transformation|GetWorldLocation _staticmesh)))
    (:else)))

(fn Lookat
  (return "" ""))